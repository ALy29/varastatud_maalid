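; Quiz HUD that runs a question sequence and shows the final score.
; BeginPlay creates the question and scorecard widgets, enables UI-only input with a visible cursor, then calls Restart to reset progress.
; NextQuestion counts correct answers and feeds each Question array entry to the question widget.
; Its LastIndex check skips the final entry before swapping to the scorecard, labelled "Sinu score:".
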(event `self.ReceiveBeginPlay`
  (bind _returnvalue (`GameplayStatics.GetPlayerController` 0))
  (bind _returnvalue_2 (`|CreateWidget` "/Game/Blueprints/wdg_question.wdg_question_C"))
  (bind _output_get (set `self.wdg question` _returnvalue_2))
  (`WidgetBlueprintLibrary.SetInputMode_UIOnlyEx` _returnvalue _output_get)
  (set `PlayerController.bShowMouseCursor` true _returnvalue)
  (bind _returnvalue_3 (`|CreateWidget` "/Game/Blueprints/wdg_score_card.wdg_score_card_C"))
  (set `self.scorecard` _returnvalue_3)
  (`self.Restart`))

(event `self.NextQuestion`
  (params (`Answer co` :type Boolean))
  (bind _scorecard (`self.scorecard`))
  (bind _current_question (`self.current question`))
  (if `Answer co`
    (`/Engine/EditorBlueprintResources/StandardMacros.IncrementInt` (`self.score`)
      (:`  `
        _)))
  (if (> (`KismetArrayLibrary.Array_LastIndex` (`self.Question`)) _current_question)
    (`/Game/Blueprints/wdg_question.init question` (`self.wdg question`) (`|GetArrayItem` (`self.Question`) _current_question))
    (`/Engine/EditorBlueprintResources/StandardMacros.IncrementInt` _current_question)
    (else
      (`UserWidget.AddToViewport` _scorecard 0)
      (`/Game/Blueprints/wdg_score_card.init score` _scorecard (`KismetTextLibrary.Conv_StringToText` (`KismetStringLibrary.Concat_StrStr` "Sinu score:" (`KismetStringLibrary.Conv_IntToString` (`self.score`)))))
      (`Widget.RemoveFromParent` (`self.wdg question`)))))

(event `self.Restart`
  (set `self.score` 0)
  (set `self.current question` 0)
  (`self.NextQuestion` false)
  (`Widget.RemoveFromParent` (`self.scorecard`))
  (`UserWidget.AddToViewport` (`self.wdg question`) 0))

(fn `UserConstructionScript`)